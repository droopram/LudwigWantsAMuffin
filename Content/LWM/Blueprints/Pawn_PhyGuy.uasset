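; Physics-driven player pawn for a floppy-character game, moved by swinging the left and right arms with Q/E and A/D.
; Each tick applies signed force to the held arms, caches shoulder, elbow and hand IK marker locations, and plays random rate-limited grunts when the head rises fast.
; Reset destroys the pawn and asks FloppyGM to respawn it, while any destruction reports death to that game mode.
; Helper functions freeze or release head physics.
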(event `self.ReceiveBeginPlay`
  ;[1 1 1] Init
  (`WidgetBlueprintLibrary.SetInputMode_GameOnly` (`GameplayStatics.GetPlayerController` 0)))

(event `self.ReceiveTick`
  (params (DeltaSeconds :type "Float (single-precision)"))
  ;[1 1 1] Init
  (`self.moveArms`)
  (`self.saveIKLocs`)
  (`self.PlaySoundEffects`))

(event `Key|D`
  (params (Key :type "Key Structure"))
  ;[1 1 1] Player  Input
  (:`Pressed`
    (set `self.swingRight` true)
    (set `self.direction` 1.0 :!label _label))
  (:`Released`
    (set `self.swingRight` false)
    (goto _label)))

(event `Key|E`
  (params (Key :type "Key Structure"))
  ;[1 1 1] Player  Input
  (:`Pressed`
    (set `self.swingLeft` true)
    (set `self.direction` 1.0 :!label _label_2))
  (:`Released`
    (set `self.swingLeft` false)
    (goto _label_2)))

(event `Key|A`
  (params (Key :type "Key Structure"))
  ;[1 1 1] Player  Input
  (:`Pressed`
    (set `self.swingRight` true)
    (set `self.direction` -1.0 :!label _label_3))
  (:`Released`
    (set `self.swingRight` false)
    (goto _label_3)))

(event `Key|Q`
  (params (Key :type "Key Structure"))
  ;[1 1 1] Player  Input
  (:`Pressed`
    (set `self.swingLeft` true)
    (set `self.direction` -1.0 :!label _label_4))
  (:`Released`
    (set `self.swingLeft` false)
    (goto _label_4)))

(event `InputAction|Reset`
  (params (Key :type "Key Structure"))
  ;[1 1 1] Player  Input
  (:`Pressed`
    (`self.callRestartPlayer`)))

(event `self.ReceiveDestroyed`
  ;[1 1 1] Handle Death
  (bind _asfloppy_gm (cast `/Game/LWM/Blueprints/FloppyGM` (`GameplayStatics.GetGameMode`)))
  (`/Game/LWM/Blueprints/FloppyGM.OnPlayerDied` _asfloppy_gm self))

(fn `callRestartPlayer`
  (locals (ControllerRef :type "Controller Object Reference"))
  (set `local.ControllerRef` (`self.GetController`))
  (`self.K2_DestroyActor`)
  (bind _asfloppy_gm (cast `/Game/LWM/Blueprints/FloppyGM` (`GameplayStatics.GetGameMode`)))
  (`GameModeBase.RestartPlayer` _asfloppy_gm (`local.ControllerRef`)))

(fn `CheckPalmDistance`
  (params (HandObject :type "SceneComponent Object Reference") (DistanceToFloor :type "Float (double-precision)"))
  (bind _handobject (`local.HandObject`))
  (bind _returnvalue (`SceneComponent.K2_GetComponentLocation` _handobject))
  (bind (_outhit _returnvalue_2) (`KismetSystemLibrary.LineTraceSingle` :`Start` _returnvalue :`End` (+ _returnvalue (* (`SceneComponent.GetUpVector` _handobject) DistanceToFloor)) :`TraceChannel` "TraceTypeQuery1" :`DrawDebugType` "ForOneFrame"))
  (if (not _returnvalue_2)
    (`SceneComponent.K2_SetRelativeRotation` :`self` (`local.HandObject`))))

(fn `firstStart`
  (`PrimitiveComponent.SetSimulatePhysics` (`self.Head`) true))

(fn `freezeHead`
  (`PrimitiveComponent.SetSimulatePhysics` (`self.Head`) false))

(fn `moveArms`
  (`|ExecutionSequence`
    (:`then_0`
      (if (`self.swingRight`)
        (`PrimitiveComponent.AddForceAtLocation` (`self.rightArm`) (* (`self.moveForce`) (`self.direction`)) (0.0 0.0 0.0) "None")))
    (:`then_1`
      (if (`self.swingLeft`)
        (`PrimitiveComponent.AddForceAtLocation` (`self.leftArm`) (* (`self.moveForce`) (`self.direction`)) (0.0 0.0 0.0) "None")))))

(fn `PlaySoundEffects`
  (if (and (> (.z (`SceneComponent.GetComponentVelocity` (`self.Head`))) 250.0) (`self.canPlaySoundEffect`))
    (set `self.canPlaySoundEffect` false)
    (`GameplayStatics.PlaySoundAtLocation` (`KismetArrayLibrary.Array_Random` (`|MakeArray` "/Game/LWM/Audio/grunt1.grunt1" "/Game/LWM/Audio/grunt2.grunt2" "/Game/LWM/Audio/grunt3.grunt3" :!type "SoundBase Object Reference")) (0.0 0.0 0.0) (struct) 1.0 1.0 0.0 null null null)
    (`KismetSystemLibrary.K2_SetTimer` null "resetSoundEffect" (`KismetMathLibrary.RandomFloatInRange` 1.0 5.0))))

(fn `resetSoundEffect`
  (set `self.canPlaySoundEffect` true))

(fn `saveIKLocs`
  (set `self.IK_Shoulder_R_Loc` (`SceneComponent.K2_GetComponentLocation` (`self.ik_shoulder_r`)))
  (set `self.IK_Elbow_R_Loc` (`SceneComponent.K2_GetComponentLocation` (`self.ik_elbow_r`)))
  (set `self.IK_Hand_R_Loc` (`SceneComponent.K2_GetComponentLocation` (`self.ik_hand_r`)))
  (set `self.IK_Shoulder_L_Loc` (`SceneComponent.K2_GetComponentLocation` (`self.ik_shoulder_l`)))
  (set `self.IK_Elbow_L_Loc` (`SceneComponent.K2_GetComponentLocation` (`self.ik_elbow_l`)))
  (set `self.IK_Hand_L_Loc` (`SceneComponent.K2_GetComponentLocation` (`self.ik_hand_l`))))

(fn `UserConstructionScript`)